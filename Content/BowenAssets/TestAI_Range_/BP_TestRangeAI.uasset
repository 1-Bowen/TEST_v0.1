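; Ranged enemy AI character that throws projectiles at the player and is destroyed after enough bullet hits.
; When the player enters HitRange, it plays a throw montage and spawns a BP_AIProjectile at SpawnProjectile once the montage completes.
; FacePlayer and StopFacePlayer toggle smooth per-tick rotation toward the player, and SetSpeed changes walk speed.
; Each BP_Bullet hit decrements HP, destroying the actor at zero.
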(event `FacePlayer`
  (set `self.isFacePlayer` true))

(event `StopFacePlayer`
  (set `self.isFacePlayer` false))

(event `self.ReceiveTick`
  (params (DeltaSeconds :type "Float (single-precision)"))
  (set `self.Delta` DeltaSeconds)
  (if (`self.isFacePlayer`)
    (`self.K2_SetActorRotation` (`KismetMathLibrary.RInterpTo` (`self.K2_GetActorRotation`) (`KismetMathLibrary.FindLookAtRotation` (`self.K2_GetActorLocation`) (`self.K2_GetActorLocation` (`GameplayStatics.GetPlayerCharacter` 0))) (`self.Delta`) 2.0))))

(event `self.ReceiveHit`
  (params (MyComp :type "PrimitiveComponent Object Reference") (Other :type "Actor Object Reference") (OtherComp :type "PrimitiveComponent Object Reference") (bSelfMoved :type Boolean) (HitLocation :type "Vector Structure") (HitNormal :type "Vector Structure") (NormalImpulse :type "Vector Structure") (Hit :type "HitResult Structure (by ref)"))
  (cast `/Game/BowenAssets/BP_Bullet` Other)
  (bind _result (`/Engine/EditorBlueprintResources/StandardMacros.DecrementInt` (`self.HP`))
    (:`  `
      (if (== _result 0)
        (`self.K2_DestroyActor`)))))

(event `self.hit range.OnComponentBeginOverlap`
  (params (OverlappedComponent :type "PrimitiveComponent Object Reference") (OtherActor :type "Actor Object Reference") (OtherComp :type "PrimitiveComponent Object Reference") (OtherBodyIndex :type Integer) (bFromSweep :type Boolean) (SweepResult :type "HitResult Structure (by ref)"))
  (cast `/Game/BowenAssets/BP_BowenPlayer` OtherActor)
  (if (not (`self.isThrow`))
    (set `self.isThrow` true)
    (`|PlayMontage` (`self.Mesh`) "/Game/BowenAssets/TestAI_Range_/TestRangedAI_Throw_Montage.TestRangedAI_Throw_Montage"
      (:`OnCompleted`
        (set `self.isThrow` false)
        (`self.ShootPlayer`)))))

(event `self.hit range.OnComponentHit`
  (params (HitComponent :type "PrimitiveComponent Object Reference") (OtherActor :type "Actor Object Reference") (OtherComp :type "PrimitiveComponent Object Reference") (NormalImpulse :type "Vector Structure") (Hit :type "HitResult Structure (by ref)")))

(fn `Set Speed`
  (params (Speed :type "Float (double-precision)"))
  (set `CharacterMovementComponent.MaxWalkSpeed` Speed (`self.CharacterMovement`)))

(fn `ShootPlayer`
  (`|SpawnActorFromClass` "/Game/BowenAssets/TestAI_Range_/BP_AIProjectile.BP_AIProjectile_C" (`SceneComponent.K2_GetComponentToWorld` (`self.spawn projectile`)) "Undefined" "OverrideRootScale" null null))

(fn `UserConstructionScript`)